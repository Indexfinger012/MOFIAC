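; AC_LockOn is an actor component that holds combat state for its owner: health, player state tag, current anim data and lock-on enemy.
; PlayHitMontage subtracts damage, then either ragdolls the owner at zero health or plays AM_HitReact, tagging HitReact and returning to Idle on completion.
; Getters and setters expose the state; SetLockOnEnemy also sets LockedOn, which becomes false for a valid enemy and true otherwise.
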(event `PlayHitMontage`
  (params (Damage :type "Float (double-precision)"))
  (bind _returnvalue (`Actor.GetComponentByClass` (`self.GetOwner`) "/Script/Engine.SkeletalMeshComponent"))
  (bind _output_get (set `self.Health` (- (`self.Health`) Damage)))
  (if (<= _output_get 0.0)
    (`PrimitiveComponent.SetSimulatePhysics` (`Character.Mesh` (cast `Character` (`self.GetOwner`) :!pure true)) true)
    (else
      (`/Engine/EditorBlueprintResources/StandardMacros.IsValid` _returnvalue
        (:`Is Valid`
          (`|PlayMontage` _returnvalue "/Game/Characters/Danny/AnimMontages/AM_HitReact.AM_HitReact"
            (:`then`
              (`self.SetTag` (`BlueprintGameplayTagLibrary.MakeLiteralGameplayTag` (struct :`TagName` "PlayerStates.HitReact")))
              (`/Engine/EditorBlueprintResources/StandardMacros.IsValid` null))
            (:`OnCompleted`
              (`self.SetTag` (`BlueprintGameplayTagLibrary.MakeLiteralGameplayTag` (struct :`TagName` "PlayerStates.Idle"))))))))))

(fn `GetAnimData`
  (returns (CurrAnimData :type "/Game/CombatSystem/Data/S_AnimData Structure"))
  (return (`self.CurrAnimData`)))

(fn `GetLockOnEnemy`
  (returns (LockOnEnemy :type "Actor Object Reference"))
  (return (`self.LockOnEnemy`)))

(fn `GetTag`
  (returns (PlayerStateTag :type "GameplayTag Structure"))
  (return (`self.PlayerStateTag`)))

(fn `SetAnimData`
  (params (CurrAnimData :type "/Game/CombatSystem/Data/S_AnimData Structure"))
  (set `self.CurrAnimData` CurrAnimData)
  (return))

(fn `SetLockOnEnemy`
  (params (LockOnEnemy :type "Actor Object Reference"))
  (bind _output_get (set `self.LockOnEnemy` LockOnEnemy))
  (`/Engine/EditorBlueprintResources/StandardMacros.IsValid` _output_get
    (:`Is Valid`
      (set `self.LockedOn?` false)
      (return))
    (:`Is Not Valid`
      (set `self.LockedOn?` true)
      (return))))

(fn `SetTag`
  (params (PlayerStateTag :type "GameplayTag Structure"))
  (set `self.PlayerStateTag` PlayerStateTag)
  (return))