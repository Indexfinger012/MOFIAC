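; AC_Director is a combat director component that tracks registered enemies and is meant to pick which one attacks the player.
; Adding an enemy starts a looping timer, its interval randomized once between bounds, and removing the last one clears it.
; Each tick counts enemies whose AC_EnemyComp flags an attack, then flags a random one only if that count is below zero, which as written never happens.
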(fn `AddEnemy`
  (params (EnemyRef :type "/Game/CombatSystem/AIs/Enemies/BP_EnemyBase Object Reference (by ref)"))
  (`KismetArrayLibrary.Array_AddUnique` (`self.EnemiesRef`) EnemyRef)
  (if (and (> (`KismetArrayLibrary.Array_Length` (`self.EnemiesRef`)) 0) (not (`KismetSystemLibrary.K2_IsTimerActiveHandle` (`self.CheckIfPlayerAttacked_TH`))))
    (bind _returnvalue (`KismetSystemLibrary.K2_SetTimer` null "CheckIfPlayerAttacked" (`KismetMathLibrary.RandomFloatInRange` 2.0 5.0) true true))
    (set `self.CheckIfPlayerAttacked_TH` _returnvalue)))

(fn `CheckIfPlayerAttacked`
  (locals (ChooseAttackingAI :type Integer))
  (bind _enemiesref (`self.EnemiesRef`))
  (bind _returnvalue (`Actor.GetComponentByClass` (`KismetArrayLibrary.Array_Random` (`self.EnemiesRef`)) "/Game/CombatSystem/Componenets/AC_EnemyComp.AC_EnemyComp_C"))
  (set `local.ChooseAttackingAI` 0)
  (if (`KismetArrayLibrary.Array_IsValidIndex` _enemiesref)
    (for _array_element _enemiesref
      (`/Engine/EditorBlueprintResources/StandardMacros.IsValid` _array_element
        (:`Is Valid`
          (bind _returnvalue_2 (`Actor.GetComponentByClass` _array_element "/Game/CombatSystem/Componenets/AC_EnemyComp.AC_EnemyComp_C"))
          (`/Engine/EditorBlueprintResources/StandardMacros.IsValid` _returnvalue_2
            (:`Is Valid`
              (if (`/Game/CombatSystem/Componenets/AC_EnemyComp.GetAttackPlayer` _returnvalue_2)
                (`/Engine/EditorBlueprintResources/StandardMacros.IncrementInt` (`local.ChooseAttackingAI`))))))))
    (if (< (`local.ChooseAttackingAI`) 0)
      (`/Engine/EditorBlueprintResources/StandardMacros.IsValid` _returnvalue
        (:`Is Valid`
          (`/Game/CombatSystem/Componenets/AC_EnemyComp.SetAttackPlayer` _returnvalue true))))))

(fn `RemoveEnemy`
  (params (EnemyRef :type "/Game/CombatSystem/AIs/Enemies/BP_EnemyBase Object Reference (by ref)"))
  (`KismetArrayLibrary.Array_RemoveItem` (`self.EnemiesRef`) EnemyRef)
  (if (<= (`KismetArrayLibrary.Array_Length` (`self.EnemiesRef`)) 0)
    (`KismetSystemLibrary.K2_ClearAndInvalidateTimerHandle` (`self.CheckIfPlayerAttacked_TH`))))