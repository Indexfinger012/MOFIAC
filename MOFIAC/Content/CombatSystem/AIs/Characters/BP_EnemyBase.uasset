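; Base enemy character for the combat system, linking AI perception to the player's combat director and the AI Blackboard.
; Sighting the player cancels the target-check timer, registers the enemy with the player's AC_Director and sets TargetActor; losing the player starts that timer.
; A text render shows "Attacking" while the enemy component flags an attack.
; On death it launches upward and is destroyed after a short delay.
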(event `self.ReceiveTick`
  (params (DeltaSeconds :type "Float (single-precision)"))
  (bind _ac_enemycomp (`self.AC_EnemyComp`)
    (:`then`
      (`TextRenderComponent.K2_SetText` (`self.TextRender`) (`KismetMathLibrary.SelectText` "Attacking" "" (`/Game/CombatSystem/Componenets/AC_EnemyComp.GetAttackPlayer` _ac_enemycomp))))
    (:`else`)))

(event `self.AIPerception.OnTargetPerceptionUpdated`
  (params (Actor :type "Actor Object Reference") (Stimulus :type "AIStimulus Structure"))
  (bind _returnvalue (`AIBlueprintHelperLibrary.GetBlackboard` null))
  (bind _returnvalue_2 (`self.GetComponentByClass` Actor "/Game/CombatSystem/Componenets/AC_Director.AC_Director_C"))
  (if (== Actor (`GameplayStatics.GetPlayerCharacter` 0))
    (if (`.bSuccessfullySensed` (break `AIStimulus` Stimulus))
      (`KismetSystemLibrary.K2_ClearAndInvalidateTimerHandle` (`self.TargetCheckerTH`))
      (`/Engine/EditorBlueprintResources/StandardMacros.IsValid` _returnvalue_2
        (:`Is Valid`
          (`/Game/CombatSystem/Componenets/AC_Director.AddEnemy` _returnvalue_2 self))
        (:`Is Not Valid`
          _))
      (`/Engine/EditorBlueprintResources/StandardMacros.IsValid` _returnvalue
        (:`Is Valid`
          (`BlackboardComponent.SetValueAsObject` _returnvalue "TargetActor" Actor)))
      (else
        (bind _returnvalue_3 (`KismetSystemLibrary.K2_SetTimer` null))
        (set `self.TargetCheckerTH` _returnvalue_3)))))

(event `Die`
  (`self.LaunchCharacter` (0.0 0.0 1000.0))
  (`KismetSystemLibrary.Delay` 3.0)
  (`self.K2_DestroyActor`))

(fn `UserConstructionScript`)