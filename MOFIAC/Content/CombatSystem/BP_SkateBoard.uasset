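; BP_SkateBoard is a combat skateboard Blueprint that damages enemies it overlaps.
; When component F begins overlapping a BP_EnemyBase, it launches the enemy along the scaled enemy-to-board vector, so toward the board, adding to existing velocity.
; It then subtracts fixed damage directly from the enemy's Health and calls Die at zero or below, printing launch vector and health for debugging.
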(event `self.f.OnComponentBeginOverlap`
  (params (OverlappedComponent :type "PrimitiveComponent Object Reference") (OtherActor :type "Actor Object Reference") (OtherComp :type "PrimitiveComponent Object Reference") (OtherBodyIndex :type Integer) (bFromSweep :type Boolean) (SweepResult :type "HitResult Structure (by ref)"))
  (bind _asbp_enemy_base (cast `/Game/CombatSystem/AIs/Characters/BP_EnemyBase` OtherActor))
  (bind _returnvalue (* (- (`self.K2_GetActorLocation`) (`self.K2_GetActorLocation` _asbp_enemy_base)) (2.0 2.0 2.0)))
  (`KismetSystemLibrary.PrintString` (`KismetStringLibrary.Conv_VectorToString` _returnvalue))
  (`Character.LaunchCharacter` _asbp_enemy_base _returnvalue false false)
  (bind _output_get (set `/Game/CombatSystem/AIs/Characters/BP_EnemyBase.Health` (- (`/Game/CombatSystem/AIs/Characters/BP_EnemyBase.Health` _asbp_enemy_base) 25) _asbp_enemy_base))
  (`KismetSystemLibrary.PrintString` (`KismetStringLibrary.Conv_IntToString` _output_get))
  (if (<= _output_get 0)
    (`/Game/CombatSystem/AIs/Characters/BP_EnemyBase.Die` _asbp_enemy_base)))

(fn `UserConstructionScript`)