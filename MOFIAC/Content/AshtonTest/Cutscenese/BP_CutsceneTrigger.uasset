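; BP_CutsceneTrigger is a trigger volume that plays a one-time cutscene when the player walks into it.
; When BP_ThirdPersonCharacter overlaps the Box, Play sets the Played flag, pauses the game and adds a W_Cutscene widget to the viewport.
; The trigger passes its PageNumber to the widget and does not unpause the game itself.
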(event `self.Box.OnComponentBeginOverlap`
  (params (OverlappedComponent :type "PrimitiveComponent Object Reference") (OtherActor :type "Actor Object Reference") (OtherComp :type "PrimitiveComponent Object Reference") (OtherBodyIndex :type Integer) (bFromSweep :type Boolean) (SweepResult :type "HitResult Structure (by ref)"))
  (if (not (`self.Played?`))
    (cast `/Game/ThirdPerson/Blueprints/BP_ThirdPersonCharacter` OtherActor)
    (`self.Play`)))

(event `Play`
  (set `self.Played?` true)
  (`GameplayStatics.SetGamePaused` true)
  (bind _returnvalue (`|CreateWidget` "/Game/AshtonTest/Cutscenese/W_Cutscene.W_Cutscene_C"))
  (set `/Game/AshtonTest/Cutscenese/W_Cutscene.PageNumber` (`self.PageNumber`) _returnvalue)
  (`UserWidget.AddToViewport` _returnvalue 0))

(fn `UserConstructionScript`)